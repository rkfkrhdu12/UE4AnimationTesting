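; Player character Blueprint that handles movement, look and dash input, and assigns two fire animation montages on BeginPlay.
; Move axes forward to MoveForward and MoveRight functions not defined here; Turn adds controller yaw, while LookUp pitches only the camera arm, without clamping.
; The Shield_Dash press applies a large fixed impulse along the normalized velocity.
; A separate force-based Dash function using DashForce is not called in this graph.
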(event `self.ReceiveBeginPlay`
  (set `self.FireAnimMontage` (`self.FireAnimation`))
  (set `self.Fire2AnimMontage` (`self.Fire2Animation`)))

(event `InputAction|Shield_Dash`
  (params (Key :type "Key Structure"))
  (:`Pressed`
    (`CharacterMovementComponent.AddImpulse` (`self.CharacterMovement`) (* (`KismetMathLibrary.Normal` (`self.GetVelocity`)) 1000000.0) false)))

(event `InputAxis|MoveForward`
  (params (AxisValue :type "Float (single-precision)"))
  (`self.MoveForward` AxisValue))

(event `InputAxis|MoveRight`
  (params (AxisValue :type "Float (single-precision)"))
  (`self.MoveRight` AxisValue))

(event `InputAxis|Turn`
  (params (AxisValue :type "Float (single-precision)"))
  (`self.AddControllerYawInput` AxisValue))

(event `InputAxis|LookUp`
  (params (AxisValue :type "Float (single-precision)"))
  (bind _cameraarmcomponent (`self.CameraArmComponent`))
  (bind (_relativerotation_roll _relativerotation_pitch _relativerotation_yaw) (`KismetMathLibrary.BreakRotator` (`SceneComponent.RelativeRotation` _cameraarmcomponent)))
  (`SceneComponent.K2_SetRelativeRotation` _cameraarmcomponent (`KismetMathLibrary.MakeRotator` _relativerotation_roll (- _relativerotation_pitch AxisValue) _relativerotation_yaw) false false))

(fn `Dash`
  (params (Direction :type "Vector Structure"))
  (`CharacterMovementComponent.AddForce` (`self.CharacterMovement`) (* Direction (`self.DashForce`))))

(fn `UserConstructionScript`)